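; Door actor for the machine room that swings open or closed when the player interacts with it.
; Interact checks a CanOpen flag, clears it and plays a metal door sound at the door mesh.
; A FlipFlop alternates playing and reversing a timeline that lerps the mesh's yaw through a quarter turn.
; The timeline's Finished output restores CanOpen, blocking new interactions mid-swing.
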(event `/Game/Code_Orange/BluePrint/Interaction_IF.Interact`
  (bind _doorr_object006 (`self.doorr_Object006`))
  (if (`self.Can_Open`)
    (set `self.Can_Open` false)
    (`GameplayStatics.PlaySoundAtLocation` "/Game/Code_Orange/audio/effect/interact/open_door/metal/open_door_metal.open_door_metal" (`SceneComponent.K2_GetComponentLocation` _doorr_object006) (struct) 1.0 1.0 0.2 null null null null)
    (`/Engine/EditorBlueprintResources/StandardMacros.FlipFlop`
      (:`A`
        (bind (_direction _newtrack_1) (`Timeline|Timeline_0` :!via `PlayFromStart` :!label _label)
          (:`Update`
            (`SceneComponent.K2_SetRelativeRotation` _doorr_object006 (`KismetMathLibrary.MakeRotator` 0.0 0.0 (`KismetMathLibrary.Lerp` 0.0 90.0 _newtrack_1)) false false))
          (:`Finished`
            (set `self.Can_Open` true))))
      (:`B`
        (goto _label :!via `Reverse`)))))

(fn `UserConstructionScript`)