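; Interactable electrical-style panel box in the machine room whose metal door swings open and closed.
; Interact plays a door sound, then a FlipFlop alternates between playing and reversing a timeline that lerps the ChestDoor yaw.
; The CanOpen flag blocks further interaction until the timeline finishes.
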(event `/Game/Code_Orange/BluePrint/Interaction_IF.Interact`
  (bind _chest_door (`self.Chest_Door`))
  (if (`self.Can_Open`)
    (set `self.Can_Open` false)
    (`GameplayStatics.PlaySoundAtLocation` "/Game/Code_Orange/audio/effect/interact/open_door/metal/open_door_metal.open_door_metal" (`SceneComponent.K2_GetComponentLocation` _chest_door) (struct) 1.0 1.0 0.2 null null null null)
    (`/Engine/EditorBlueprintResources/StandardMacros.FlipFlop`
      (:`A`
        (bind (_direction _newtrack_1) (`Timeline|Timeline_0` :!via `PlayFromStart` :!label _label)
          (:`Update`
            (`SceneComponent.K2_SetRelativeRotation` _chest_door (`KismetMathLibrary.MakeRotator` 0.0 0.0 (`KismetMathLibrary.Lerp` -180.0 -300.0 _newtrack_1)) false false))
          (:`Finished`
            (set `self.Can_Open` true))))
      (:`B`
        (goto _label :!via `Reverse`)))))

(fn `UserConstructionScript`)