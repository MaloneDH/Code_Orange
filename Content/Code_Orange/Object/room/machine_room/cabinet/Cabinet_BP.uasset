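; Interactable cabinet for the machine room, with left and right doors that swing open and closed.
; Each Interact plays a steel drawer sound and alternates via a FlipFlop between playing and reversing a timeline that lerps both doors' relative yaw.
; A CanOpen flag blocks further interaction until the timeline finishes.
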(event `/Game/Code_Orange/BluePrint/Interaction_IF.Interact`
  (if (`self.Can_Open`)
    (set `self.Can_Open` false)
    (`GameplayStatics.PlaySoundAtLocation` "/Game/Code_Orange/audio/effect/interact/open_cabinet/550411__mattruthsound__steel-drawers_06.550411__mattruthsound__steel-drawers_06" (`SceneComponent.K2_GetComponentLocation` (`self.cabinet_cabinet`)) (struct) 1.0 1.0 0.0 null null null null)
    (`/Engine/EditorBlueprintResources/StandardMacros.FlipFlop`
      (:`A`
        (bind (_direction _newtrack_0) (`Timeline|Timeline_0` :!via `PlayFromStart` :!label _label)
          (:`Update`
            (`SceneComponent.K2_SetRelativeRotation` (`self.cabinet_cabinet_door_l`) (`KismetMathLibrary.MakeRotator` 0.0 0.0 (`KismetMathLibrary.Lerp` -145.0 -45.0 _newtrack_0)) false false)
            (`SceneComponent.K2_SetRelativeRotation` (`self.cabinet_cabinet_door_r`) (`KismetMathLibrary.MakeRotator` 0.0 0.0 (`KismetMathLibrary.Lerp` 110.0 10.0 _newtrack_0)) false false))
          (:`Finished`
            (set `self.Can_Open` true))))
      (:`B`
        (goto _label :!via `Reverse`)))))

(fn `UserConstructionScript`)