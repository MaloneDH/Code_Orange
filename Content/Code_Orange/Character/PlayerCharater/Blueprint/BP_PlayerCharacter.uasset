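; Player character Blueprint handling health, death, a toggleable flashlight and object interaction.
; Damage reduces Life and plays a hurt sound, or at zero plays the death sound and montage, sets Death and disables look and move input.
; Camera line traces set CanInteract on Tick from the "Interact" component tag and send InteractMessage to the hit actor on key press.
; Check_PM traces downward for surface type but acts on no result.
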(event `self.ReceiveBeginPlay`
  (set `CharacterMovementComponent.MaxWalkSpeed` 400.0 (`self.CharacterMovement`)))

(event `self.ReceiveAnyDamage`
  (params (Damage :type "Float (single-precision)") (DamageType :type "DamageType Object Reference") (InstigatedBy :type "Controller Object Reference") (DamageCauser :type "Actor Object Reference"))
  (bind _returnvalue (`GameplayStatics.GetPlayerController` 0))
  (bind _returnvalue_2 (`self.K2_GetActorLocation`))
  (bind _life (`self.Life`))
  ;[1 0.1534 0.1136] Damaged
  (set `self.Life` (- _life Damage))
  (if (<= _life 0.0)
    (`GameplayStatics.PlaySoundAtLocation` "/Game/Code_Orange/audio/character/player/death/Player_Death_cue.Player_Death_cue" _returnvalue_2 (struct) 1.0 1.0 0.0 null null null null)
    (`self.PlayAnimMontage` "/Game/Code_Orange/Man/Demo/Animations/Death_1_Montage.Death_1_Montage")
    (set `self.Death` true)
    (`Controller.SetIgnoreLookInput` _returnvalue true)
    (`Controller.SetIgnoreMoveInput` _returnvalue true)
    (else
      (`GameplayStatics.PlaySoundAtLocation` "/Game/Code_Orange/audio/character/player/damaged/damaged.damaged" _returnvalue_2 (struct) 1.0 1.0 0.0 null null null null))))

(event `InputAction|Turn_Flashlight`
  (params (Key :type "Key Structure"))
  (bind _flashlight (`self.flashlight`))
  ;[1 1 1] Turn Flashlight
  (:`Pressed`
    (`GameplayStatics.PlaySoundAtLocation` "/Game/Code_Orange/audio/effect/turnlight.turnlight" (`self.K2_GetActorLocation`) (struct) 1.0 1.0 0.0 null null null null)
    (`/Engine/EditorBlueprintResources/StandardMacros.FlipFlop`
      (:`A`
        (`SceneComponent.SetVisibility` _flashlight true false))
      (:`B`
        (`SceneComponent.SetVisibility` _flashlight false false)))))

(event `Check_PM`
  (bind _returnvalue (`self.K2_GetActorLocation`))
  ;[1 1 1] Chk_Surface
  (bind (_outhit _returnvalue_2) (`KismetSystemLibrary.LineTraceSingle` :`Start` _returnvalue :`End` (- _returnvalue (0.0 0.0 144.0)) :`TraceChannel` "TraceTypeQuery1" :`TraceColor` (struct :`R` 1.0) :`TraceHitColor` (struct :`G` 1.0)))
  (if _returnvalue_2
    (switch `EPhysicalSurface` (`GameplayStatics.GetSurfaceType` _outhit))))

(event `self.ReceiveTick`
  (params (DeltaSeconds :type "Float (single-precision)"))
  (bind _camera (`self.Camera`))
  (bind _returnvalue (`SceneComponent.K2_GetComponentLocation` _camera))
  ;[1 1 1] Chk_Object_interact
  (bind (_outhit _returnvalue_2) (`KismetSystemLibrary.LineTraceSingle` :`Start` _returnvalue :`End` (+ _returnvalue (* (`KismetMathLibrary.GetForwardVector` (`SceneComponent.K2_GetComponentRotation` _camera)) 350.0)) :`TraceChannel` "TraceTypeQuery1" :`TraceColor` (struct :`R` 1.0) :`TraceHitColor` (struct :`G` 1.0)))
  (if _returnvalue_2
    (if (`ActorComponent.ComponentHasTag` (`.HitComponent` (`GameplayStatics.BreakHitResult` _outhit)) "Interact")
      (set `self.Can_Interact` true)
      (else
        (set `self.Can_Interact` false)))))

(event `InputAction|Interact_Object`
  (params (Key :type "Key Structure"))
  (bind _camera (`self.Camera`))
  (bind _returnvalue (`SceneComponent.K2_GetComponentLocation` _camera))
  ;[1 1 1] Object_interact
  (:`Pressed`
    (bind (_outhit _returnvalue_2) (`KismetSystemLibrary.LineTraceSingle` _returnvalue (+ _returnvalue (* (`KismetMathLibrary.GetForwardVector` (`SceneComponent.K2_GetComponentRotation` _camera)) 350.0)) "TraceTypeQuery1"))
    (if _returnvalue_2
      (message `/Game/Code_Orange/BluePrint/Interaction_IF.Interact` (`.HitActor` (`GameplayStatics.BreakHitResult` _outhit))))))

(fn `UserConstructionScript`)